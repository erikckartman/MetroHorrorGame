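; BP_Door is a door actor meant to swing 90 degrees in yaw when OpenDoor is called.
; BeginPlay caches the starting rotation and derives the opened rotation from it, and OpenDoor sets the IsOpening flag.
; Tick then applies one high-speed RInterpTo step from the cached rotation and clears the flag immediately, so the door jumps in one frame rather than animating.
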(event EventBeginPlay
  (bind _output_get (Variables|Default|SetCurrentRotation (Transformation|GetActorRotation)))
  (Variables|Default|SetOpenedRotation (Math|Rotator|MakeRotator (.Roll (Math|Rotator|BreakRotator _output_get)) (.Pitch (Math|Rotator|BreakRotator _output_get)) (- (.Yaw (Math|Rotator|BreakRotator _output_get)) 9e+01))))

(event EventTick
  (params (DeltaSeconds :type Float%20%28single-precision%29))
  (if (Variables|Default|GetIsOpening)
    (Transformation|SetActorRotation (Math|Interpolation|RInterpTo (Variables|Default|GetCurrentRotation) (Variables|Default|GetOpenedRotation) DeltaSeconds 1e+02))
    (Variables|Default|SetIsOpening false)))

(fn ConstructionScript)

(fn OpenDoor
  (Variables|Default|SetIsOpening true))